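; BP_Tockie_Repeat is a movable pawn that replays a recorded sequence of movement inputs.
; FireRecording stores the input array, moves the pawn to the given start position and starts playback.
; Each Tick consumes one "A", "N" or "D" entry as negative, zero or positive world-X movement, so replay follows frame count rather than time.
; When the array ends, playback stops, the index resets and the pawn jumps to a hardcoded location.
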(event `self.ReceiveTick`
  (params (DeltaSeconds :type "Float (single-precision)"))
  (bind _output (`|GetArrayItem` (`self.InputsToEmulate`) (`self.InputsIndex`)))
  (if (`self.PlayRecording`)
    (if (`KismetStringLibrary.EqualEqual_StrStr` _output "A")
      (`self.AddMovementInput` (1.0 0.0 0.0) -1.0)
      (bind _result (`/Engine/EditorBlueprintResources/StandardMacros.IncrementInt` (`self.InputsIndex`) :!label _label)
        (:`  `
          (`/Engine/EditorBlueprintResources/StandardMacros.CompareInt` _result (`KismetArrayLibrary.Array_Length` (`self.InputsToEmulate`))
            (:`==`
              (set `self.PlayRecording` false)
              (set `self.InputsIndex` 0)
              (`self.K2_SetActorLocation` (500.0 500.0 500.0))))))
      (elif (`KismetStringLibrary.EqualEqual_StrStr` _output "N")
        (`self.AddMovementInput` (1.0 0.0 0.0) 0.0)
        (goto _label)
        (elif (`KismetStringLibrary.EqualEqual_StrStr` _output "D")
          (`self.AddMovementInput` (1.0 0.0 0.0))
          (goto _label))))))

(event `/Game/BluePrints/BP_Record_Interface.Fire Recording`
  (params (RecordedInputs :type "Array of String (by ref)") (StartPos :type "Vector Structure"))
  (set `self.InputsToEmulate` RecordedInputs)
  (set `self.PlayRecording` true)
  (`self.K2_SetActorLocation` StartPos))

(fn `UserConstructionScript`)